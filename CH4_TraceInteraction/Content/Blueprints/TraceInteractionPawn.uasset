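; TraceInteractionPawn is a player pawn that forwards left mouse presses and releases to its TraceInteractionComponent as activate down and up calls, passing itself along.
; On BeginPlay it sets floor-level tracking origin and lets the camera follow controller rotation only when no headset is enabled.
; Without a headset, mouse movement drives yaw and inverted pitch as a monitor debug fallback for VR.
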(event EventBeginPlay
  ;[1 1 1] Debug
  (Variables|/Script/Engine.CameraComponent|SetbUsePawnControlRotation (Variables|Default|GetCamera) (not (Class|HeadMountedDisplayFunctionLibrary|IsHeadMountedDisplayEnabled)))
  (Class|HeadMountedDisplayFunctionLibrary|SetTrackingOrigin "Floor"))

(event EventActorBeginOverlap
  (params (OtherActor :type Actor%20Object%20Reference)))

(event EventTick
  (params (DeltaSeconds :type Float%20%28single-precision%29)))

(event Input|MouseEvents|MouseX
  (params (AxisValue :type Float%20%28single-precision%29))
  ;[1 1 1] Monitor Debug
  (if (not (Class|HeadMountedDisplayFunctionLibrary|IsHeadMountedDisplayEnabled))
    (Pawn|Input|AddControllerYawInput AxisValue)))

(event Input|MouseEvents|MouseY
  (params (AxisValue :type Float%20%28single-precision%29))
  ;[1 1 1] Monitor Debug
  (if (not (Class|HeadMountedDisplayFunctionLibrary|IsHeadMountedDisplayEnabled))
    (Pawn|Input|AddControllerPitchInput (* AxisValue -1.0))))

(event Input|MouseEvents|LeftMouseButton
  (params (Key :type Key%20Structure :default "AnyKey"))
  (bind _self self)
  (bind _traceinteractioncomponent (Variables|Default|GetTraceInteractionComponent))
  (:Pressed
    (Default|ActivateDown _traceinteractioncomponent _self))
  (:Released
    (Default|ActivateUp _traceinteractioncomponent _self)))

(fn ConstructionScript)