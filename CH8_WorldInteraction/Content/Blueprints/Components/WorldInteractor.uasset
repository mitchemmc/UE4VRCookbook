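; WorldInteractor is a scene component that lets its owner hover, drag, use and pick up objects in the world.
; While enabled, Tick runs a sphere overlap and tracks the first hit actor, ending any drag when it changes.
; A second gate sends drag updates each tick between start and stop.
; Targets react through interface messages and can approve pickup, which attaches them to the component until dropped.
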(event Custom|Enable
  (Utilities|FlowControl|Gate false) ; enters at Open
)

(event Custom|Pickup
  (bind _hoveredobject (Variables|Default|GetHoveredObject))
  (Utilities|IsValid _hoveredobject
    (:Is%20Valid
      (bind _pickup (Class|WorldInteractionInterface|CanPickup(Message) _hoveredobject))
      (if _pickup
        (bind _output_get (Variables|Default|SetPickedUpObject (Variables|Default|GetHoveredObject)))
        (Transformation|AttachComponentToComponent _output_get self "None" "SnapToTarget" "SnapToTarget" "KeepWorld" true)
        (Class|WorldInteractionInterface|OnPickup(Message) (Variables|Default|GetPickedUpObject) self)))))

(event Custom|Drop
  (Utilities|IsValid (Variables|Default|GetPickedUpObject)
    (:Is%20Valid
      (Transformation|DetachFromActor (Variables|Default|GetPickedUpObject) "KeepWorld" "KeepWorld" "KeepWorld")
      (Class|WorldInteractionInterface|OnDrop(Message) (Variables|Default|GetPickedUpObject) self)
      (Variables|Default|SetHoveredObject 0)
      (Variables|Default|SetPickedUpObject 0))))

(event Custom|UseHoveredObject
  (Class|WorldInteractionInterface|OnUse(Message) (Variables|Default|GetHoveredObject) self))

(event Custom|StartDrag
  (Variables|Default|SetDragging true)
  (Class|WorldInteractionInterface|OnDragStart(Message) (Variables|Default|GetHoveredObject) self)
  (Utilities|FlowControl|Gate true) ; enters at Open
)

(event Custom|StopDrag
  (if (Variables|Default|GetDragging)
    (Variables|Default|SetDragging false)
    (Class|WorldInteractionInterface|OnDragEnd(Message) (Variables|Default|GetHoveredObject) self)
    (Utilities|FlowControl|Gate true) ; enters at Close
  ))

(event Custom|Disable
  (Utilities|FlowControl|Gate false) ; enters at Close
)

(event EventTick
  (params (DeltaSeconds :type Float%20%28single-precision%29))
  (Utilities|FlowControl|Gate false
    (:Exit
      (Utilities|FlowControl|Sequence
        (:then_0
          (bind _outactors (Class|KismetSystemLibrary|SphereOverlapActorsNEW (Transformation|GetWorldLocation) (Variables|Default|GetRadius) (Utilities|Array|MakeArray "ObjectTypeQuery2" "ObjectTypeQuery4") 0 (Utilities|Array|MakeArray (Components|GetOwner))))
          (if (!= (Variables|Default|GetHoveredObject) (Utilities|Array|Get(acopy) _outactors))
            (Class|WorldInteractionInterface|OnUnhover(Message) (Variables|Default|GetHoveredObject) self)
            (CallFunction|StopDrag)
            (bind _output_get (Variables|Default|SetHoveredObject (Utilities|Array|Get(acopy) _outactors)))
            (Class|WorldInteractionInterface|OnHover(Message) _output_get self)))
        (:then_1
          (Utilities|FlowControl|Gate true
            (:Exit
              (Class|WorldInteractionInterface|OnDrag(Message) (Variables|Default|GetHoveredObject) self))))))))