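; NavMeshTeleportVolume is a trace-interactive volume that teleports a player to the pointed spot on the navmesh.
; While a trace is on it, it shows TeleportVisualizer and moves it to the hit point projected onto navigation.
; Releasing activate moves the instigator to that projected XY at the volume's own Z.
; The move adds the horizontal pawn-to-camera offset, so the camera, rather than the pawn origin, lands on the target.
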(event EventBeginPlay)

(event Collision|EventActorBeginOverlap
  (params (OtherActor :type Actor%20Object%20Reference)))

(event EventTick
  (params (DeltaSeconds :type Float%20%28single-precision%29)))

(fn ConstructionScript)

(fn TeleportPlayer
  (params (Player :type Pawn%20Object%20Reference) (Location :type Vector))
  (bind _asplayer_controller (Utilities|Casting|CastToPlayerController (Pawn|GetController Player)))
  (Transformation|SetActorLocation Player (+ (Math|Vector|MakeVector (.x (- (Transformation|GetActorLocation Player) (Camera|GetCameraLocation (Variables|/Script/Engine.PlayerController|GetPlayerCameraManager _asplayer_controller)))) (.y (- (Transformation|GetActorLocation Player) (Camera|GetCameraLocation (Variables|/Script/Engine.PlayerController|GetPlayerCameraManager _asplayer_controller)))) 0.0) Location) false false))

(fn ProjectPoint
  (params (Point :type Vector))
  (return (.ProjectedLocation (AI|Navigation|ProjectPointtoNavigation Point 0 0 "0.000000,0.000000,0.000000"))))

(fn TraceActivateDown
  (params (Hit :type Hit%20Result%20Structure) (Instigator :type Pawn%20Object%20Reference))
  (return false))

(fn TraceActivateUp
  (params (Hit :type Hit%20Result%20Structure) (Instigator :type Pawn%20Object%20Reference))
  (bind _location (Collision|BreakHitResult Hit))
  (bind _projectedpoint (CallFunction|ProjectPoint _location))
  (CallFunction|TeleportPlayer Instigator (Math|Vector|MakeVector (.x _projectedpoint) (.y _projectedpoint) (.z (Transformation|GetActorLocation))))
  (return false))

(fn TraceHitComponent
  (params (Hit :type Hit%20Result%20Structure) (Component :type Primitive%20Component%20Object%20Reference))
  (return false))

(fn TraceHitObject
  (params (Hit :type Hit%20Result%20Structure))
  (Rendering|SetVisibility (Variables|Default|GetTeleportVisualizer) true true)
  (return false))

(fn TraceLeaveComponent
  (params (Hit :type Hit%20Result%20Structure) (Component :type Primitive%20Component%20Object%20Reference))
  (return false))

(fn TraceLeaveObject
  (params (Hit :type Hit%20Result%20Structure))
  (Rendering|SetVisibility (Variables|Default|GetTeleportVisualizer) false true)
  (return false))

(fn TraceMove
  (params (Hit :type Hit%20Result%20Structure%20%28by%20ref%29))
  (Transformation|SetWorldLocation (Variables|Default|GetTeleportVisualizer) (CallFunction|ProjectPoint (.Location (Collision|BreakHitResult Hit))) false false)
  (return false))