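; GlobalMenu is a HUD for Gear VR that opens the Oculus global menu when the back button is held.
; BeginPlay enables input and disables Gear VR's built-in back-button handling.
; Pressing Android Back or K starts a 0.75-second timer that calls OpenMenu, and releasing clears it.
; While the timer runs, DrawHUD draws a centered circle material whose PercentComplete parameter follows the elapsed time.
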(event EventBeginPlay
  (bind _returnvalue (Game|Player|GetOwningPlayerController))
  (Input|EnableInput _returnvalue)
  (Development|ExecuteConsoleCommand "gearvr.handlebackbutton 0" _returnvalue)
  (bind _returnvalue_2 (Rendering|Material|CreateDynamicMaterialInstance "/Game/Materials/UICircle.UICircle" :!class /Script/Engine.KismetMaterialLibrary))
  (Variables|Default|SetCircleMat _returnvalue_2))

(event EventDrawHUD
  (params (SizeX :type Integer) (SizeY :type Integer))
  (bind _circleradius (Variables|Default|GetCircleRadius))
  (bind _returnvalue (* _circleradius 2.0))
  (if (Utilities|Time|IsTimerActivebyHandle (Variables|Default|GetBackButtonTimer))
    (Rendering|Material|SetScalarParameterValue (Variables|Default|GetCircleMat) "PercentComplete" (/ (Class|KismetSystemLibrary|GetTimerElapsedTimeHandle (Variables|Default|GetBackButtonTimer)) 0.75) :!class /Script/Engine.MaterialInstanceDynamic)
    (Canvas|DrawMaterial (Variables|Default|GetCircleMat) (- (* SizeX 0.5) (Variables|Default|GetCircleRadius)) (- (* SizeY 0.5) (Variables|Default|GetCircleRadius)) _returnvalue _returnvalue 0.0 0.0 1.0 1.0 1.0)))

(event Input|KeyboardEvents|AndroidBack
  (params (Key :type Key%20Structure :default "AnyKey"))
  (:Pressed
    (bind _returnvalue (Utilities|Time|SetTimerbyFunctionName 0 "OpenMenu" 0.75))
    (Variables|Default|SetBackButtonTimer _returnvalue))
  (:Released
    (Class|KismetSystemLibrary|ClearTimerHandle (Variables|Default|GetBackButtonTimer))))

(event Input|KeyboardEvents|K
  (params (Key :type Key%20Structure :default "AnyKey"))
  (:Pressed
    (bind _returnvalue (Utilities|Time|SetTimerbyFunctionName 0 "OpenMenu" 0.75))
    (Variables|Default|SetBackButtonTimer _returnvalue))
  (:Released
    (Class|KismetSystemLibrary|ClearTimerHandle (Variables|Default|GetBackButtonTimer))))

(fn ConstructionScript)

(fn OpenMenu
  (Development|ExecuteConsoleCommand "OVRGLOBALMENU"))