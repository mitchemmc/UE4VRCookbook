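; A world-space menu actor whose widget component shows a start, difficulty and exit menu operated through trace events.
; On BeginPlay it casts the widget to MenuWidget and binds its controls: start and difficulty changes only print messages, while exit quits the game.
; Trace move feeds the hit result into a Widget Interaction component as a custom hit, and trace activate down/up press and release the left mouse button on it.
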(event Custom|StartButtonClicked_Event
  (Development|PrintString "Open Level"))

(event Custom|ExitButtonClicked_Event
  (Game|QuitGame 0 "Quit"))

(event Custom|DifficultyChanged_Event
  (params (SelectedItem :type String) (SelectionType :type ESelectInfo%20Enum))
  (Development|PrintString (Utilities|String|Append "Difficulty changed to: " SelectedItem)))

(event EventBeginPlay
  (bind _asmenu_widget (Utilities|Casting|CastToMenuWidget (UserInterface|GetUserWidgetObject (Variables|Default|GetWidget))))
  (bind _output_get (Variables|Default|SetWidgetObject _asmenu_widget))
  (EventDispatchers|AssignOnClicked (Variables|/Game/UMG/MenuWidget.MenuWidget_C|GetStartButton _output_get) (delegate Custom|StartButtonClicked_Event))
  (EventDispatchers|AssignOnSelectionChanged (Variables|/Game/UMG/MenuWidget.MenuWidget_C|GetDifficultyCombo _output_get) (delegate Custom|DifficultyChanged_Event))
  (EventDispatchers|AssignOnClicked (Variables|/Game/UMG/MenuWidget.MenuWidget_C|GetExitButton _output_get) (delegate Custom|ExitButtonClicked_Event)))

(fn ConstructionScript)

(fn TraceActivateDown
  (params (Hit :type Hit%20Result%20Structure) (Instigator :type Pawn%20Object%20Reference))
  (Class|WidgetInteractionComponent|PressPointerKey (Variables|Default|GetWidgetInteraction) "LeftMouseButton")
  (return false))

(fn TraceActivateUp
  (params (Hit :type Hit%20Result%20Structure) (Instigator :type Pawn%20Object%20Reference))
  (Class|WidgetInteractionComponent|ReleasePointerKey (Variables|Default|GetWidgetInteraction) "LeftMouseButton")
  (return false))

(fn TraceHitComponent
  (params (Hit :type Hit%20Result%20Structure) (Component :type Primitive%20Component%20Object%20Reference))
  (return false))

(fn TraceHitObject
  (params (Hit :type Hit%20Result%20Structure))
  (return false))

(fn TraceLeaveComponent
  (params (Hit :type Hit%20Result%20Structure) (Component :type Primitive%20Component%20Object%20Reference))
  (return false))

(fn TraceLeaveObject
  (params (Hit :type Hit%20Result%20Structure))
  (return false))

(fn TraceMove
  (params (Hit :type Hit%20Result%20Structure%20%28by%20ref%29))
  (Class|WidgetInteractionComponent|SetCustomHitResult (Variables|Default|GetWidgetInteraction) Hit)
  (return false))