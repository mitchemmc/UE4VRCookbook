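; MenuActor is an actor hosting a main menu widget with start, difficulty and exit controls.
; On BeginPlay it casts its widget component's object to MenuWidget and binds the button clicks and the combo box selection change.
; Start and difficulty changes only print placeholder messages, while Exit quits the game.
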(event Custom|StartButtonClicked_Event
  (Development|PrintString "Open Level"))

(event Custom|ExitButtonClicked_Event
  (Game|QuitGame 0 "Quit"))

(event Custom|DifficultyChanged_Event
  (params (SelectedItem :type String) (SelectionType :type ESelectInfo%20Enum))
  (Development|PrintString (Utilities|String|Append "Difficulty changed to: " SelectedItem)))

(event EventBeginPlay
  (bind _asmenu_widget (Utilities|Casting|CastToMenuWidget (UserInterface|GetUserWidgetObject (Variables|Default|GetWidget))))
  (bind _output_get (Variables|Default|SetWidgetObject _asmenu_widget))
  (EventDispatchers|AssignOnClicked (Variables|/Game/UMG/MenuWidget.MenuWidget_C|GetStartButton _output_get) (delegate Custom|StartButtonClicked_Event))
  (EventDispatchers|AssignOnSelectionChanged (Variables|/Game/UMG/MenuWidget.MenuWidget_C|GetDifficultyCombo _output_get) (delegate Custom|DifficultyChanged_Event))
  (EventDispatchers|AssignOnClicked (Variables|/Game/UMG/MenuWidget.MenuWidget_C|GetExitButton _output_get) (delegate Custom|ExitButtonClicked_Event)))

(fn ConstructionScript)