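; TraceComponentPawn1 is a VR-capable pawn that hosts a trace interaction component, with a desktop mouse-look fallback for debugging.
; On BeginPlay it passes its widget interaction to the component and sets floor-level tracking.
; Left mouse press and release drive the component's activate down and up calls.
; Without an enabled headset, the camera follows control rotation and mouse axes turn the view.
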(event EventBeginPlay
  ;[1 1 1] Setup Trace Interaction Component
  (Default|Setup (Variables|Default|GetTraceInteractionComponent1) (Variables|Default|GetWidgetInteraction))
  ;[1 1 1] Debug
  (Variables|/Script/Engine.CameraComponent|SetbUsePawnControlRotation (Variables|Default|GetCamera) (not (Class|HeadMountedDisplayFunctionLibrary|IsHeadMountedDisplayEnabled)))
  (Class|HeadMountedDisplayFunctionLibrary|SetTrackingOrigin "Floor"))

(event Input|MouseEvents|MouseX
  (params (AxisValue :type Float%20%28single-precision%29))
  ;[1 1 1] Monitor Debug
  (if (not (Class|HeadMountedDisplayFunctionLibrary|IsHeadMountedDisplayEnabled))
    (Pawn|Input|AddControllerYawInput AxisValue)))

(event Input|MouseEvents|MouseY
  (params (AxisValue :type Float%20%28single-precision%29))
  ;[1 1 1] Monitor Debug
  (if (not (Class|HeadMountedDisplayFunctionLibrary|IsHeadMountedDisplayEnabled))
    (Pawn|Input|AddControllerPitchInput (* AxisValue -1.0))))

(event Input|MouseEvents|LeftMouseButton
  (params (Key :type Key%20Structure :default "AnyKey"))
  (bind _self self)
  (bind _traceinteractioncomponent1 (Variables|Default|GetTraceInteractionComponent1))
  ;[1 1 1] Activate Trace Interaction Component on mouse click
  (:Pressed
    (Default|ActivateDown _traceinteractioncomponent1 _self))
  (:Released
    (Default|ActivateUp _traceinteractioncomponent1 _self)))

(fn ConstructionScript)